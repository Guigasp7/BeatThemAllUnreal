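; Player character Blueprint for a beat 'em up, managing health, combo state, jump state, game over and respawn.
; It creates health bar and combo counter widgets, updating the health bar on damage.
; Notify handlers advance or reset the combo step and toggle the action lock, with jumping using a separate step and montages.
; GameOver disables movement and shows a UI-only game over screen, while Respawn reloads the current level.
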(event Custom|On%20ResetCombo%20Notify
  (if (Variables|Default|GetIsJumping)
    (Variables|Default|SetComboStep 4)
    (else
      (Variables|Default|SetComboStep 0)))
  (Variables|Default|SetActionLocked false))

(event Custom|On%20CanCombo%20Notify
  (if (Variables|Default|GetIsJumping)
    _
    (elif (<= (Variables|Default|GetComboStep) 2)
      (Variables|Default|SetComboStep (+ (Variables|Default|GetComboStep) 1))))
  (Variables|Default|SetActionLocked false))

(event Custom|On%20ResetComboCounter%20Notify
  (Variables|Default|SetComboCounter 0)
  (Variables|Default|SetActionLocked true))

(event Custom|On%20EndDamageAnim%20Notify
  (Variables|Default|SetActionLocked false))

(event Custom|InitializeHealth
  (bind _maxhealth (Variables|Default|GetMaxHealth))
  (bind _output_get (Variables|Default|SetCurrentHealth _maxhealth))
  (Default|UpdateHealthBar (Variables|Default|GetUI_HealthBar) _output_get _maxhealth))

(event Custom|GameOver
  (bind _returnvalue (Game|GetPlayerController 0))
  (bind _charactermovement (Variables|Character|GetCharacterMovement))
  (Components|Movement|StopMovementImmediately _charactermovement)
  (Pawn|Components|CharacterMovement|DisableMovement _charactermovement)
  (Utilities|FlowControl|Delay 1.0)
  (bind _returnvalue_2 (UserInterface|CreateWidget "/Game/BeatThemAll/Blueprints/UI_GameOverScreen.UI_GameOverScreen_C"))
  (bind _output_get (Variables|Default|SetUI_GameOver _returnvalue_2))
  (UserInterface|Viewport|AddtoViewport _output_get 0)
  (Variables|/Script/Engine.PlayerController|SetbShowMouseCursor _returnvalue true)
  (Input|SetInputModeUIOnly _returnvalue _returnvalue_2 "DoNotLock" false))

(event Custom|Respawn
  (bind _returnvalue (Game|GetPlayerController 0))
  (Variables|Default|SetIsDead false)
  (bind _returnvalue_2 (Game|GetCurrentLevelName true))
  (Game|OpenLevel(byName) (Utilities|String|StringToName _returnvalue_2))
  (Variables|/Script/Engine.PlayerController|SetbShowMouseCursor _returnvalue false)
  (Input|SetInputModeGameOnly _returnvalue false)
  (CallFunction|InitializeHealth))

(event EventBeginPlay
  (bind _returnvalue (UserInterface|CreateWidget "/Game/BeatThemAll/Blueprints/UI_PlayerHealth.UI_PlayerHealth_C"))
  (bind _output_get (Variables|Default|SetUI_HealthBar _returnvalue))
  (UserInterface|Viewport|AddtoViewport _output_get 0)
  (CallFunction|InitializeHealth)
  (bind _returnvalue_2 (UserInterface|CreateWidget "/Game/BeatThemAll/Blueprints/UI_ComboCounter.UI_ComboCounter_C"))
  (bind _output_get_2 (Variables|Default|SetUI_ComboCounter _returnvalue_2))
  (UserInterface|Viewport|AddtoViewport _output_get_2 0))

(event Game|Damage|EventAnyDamage
  (params (Damage :type Float%20%28single-precision%29) (DamageType :type Damage%20Type%20Object%20Reference) (InstigatedBy :type Controller%20Object%20Reference) (DamageCauser :type Actor%20Object%20Reference))
  (bind _output_get (Variables|Default|SetCurrentHealth (- (Variables|Default|GetCurrentHealth) Damage)))
  (Class|PlayerCharacter|Damaged)
  (Default|UpdateHealthBar (Variables|Default|GetUI_HealthBar) _output_get (Variables|Default|GetMaxHealth)))

(event EventTick
  (params (DeltaSeconds :type Float%20%28single-precision%29)))

(event EventOnJumped
  (Variables|Default|SetIsJumping true)
  (Variables|Default|SetComboStep 4)
  (Variables|Default|SetActionLocked true)
  (Animation|Montage|PlayMontage (Variables|Character|GetMesh) "/Game/BeatThemAll/AnimationMontages/AM_JumpStart.AM_JumpStart" 1.0 0.0 "Default"
    (:then
      (Variables|Default|SetActionLocked false))))

(event EventOnLanded
  (params (Hit :type Hit%20Result%20Structure%20%28by%20ref%29))
  (Variables|Default|SetIsJumping false)
  (Variables|Default|SetComboStep 0)
  (Animation|Montage|PlayMontage 0 "/Game/BeatThemAll/AnimationMontages/AM_JumpLand.AM_JumpLand"))

(fn ConstructionScript)